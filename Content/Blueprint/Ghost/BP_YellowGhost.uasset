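; Yellow ghost for a Pac-Man-style game, handling the visual and collision side of its alive, dead and fear modes.
; Each mode event swaps the GhostVisual mesh between the orange ghost, eyes and scared ghost.
; The events also set the capsule's collision profile, so the dead ghost ignores pawns while alive and scared ghosts use the standard Pawn profile.
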(event EventSetAliveModeBP
  (Components|StaticMesh|SetStaticMesh (Variables|Default|GetGhostVisual) "/Game/Assets/pac-man_assests_orange_ghost.pac-man_assests_orange_ghost")
  (Collision|SetCollisionProfileName (Variables|Default|GetCapsuleComponent) "Pawn" true :!class /Script/Engine.PrimitiveComponent))

(event EventSetDeadModeBP
  (Components|StaticMesh|SetStaticMesh (Variables|Default|GetGhostVisual) "/Game/Assets/GhostEye.GhostEye")
  (Collision|SetCollisionProfileName (Variables|Default|GetCapsuleComponent) "IgnoreOnlyPawn" true :!class /Script/Engine.PrimitiveComponent))

(event EventSetFearModeBP
  (Components|StaticMesh|SetStaticMesh (Variables|Default|GetGhostVisual) "/Game/Assets/pac-man_assests_scared_ghost.pac-man_assests_scared_ghost")
  (Collision|SetCollisionProfileName (Variables|Default|GetCapsuleComponent) "Pawn" true :!class /Script/Engine.PrimitiveComponent))

(fn ConstructionScript)