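; Behavior tree task, named for Pinky, that moves the AI pawn toward a Blackboard location within a stop distance.
; IsAsyncrone selects AIMoveTo, which targets the location scaled by 1.5 and finishes on arrival or failure.
; Otherwise MoveToLocation requests a move to the unscaled location and finishes immediately, counting Already at Goal as failure.
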(event EventReceiveExecuteAI
  (params (OwnerController :type AI%20Controller%20Object%20Reference) (ControlledPawn :type Pawn%20Object%20Reference))
  (if (Variables|Default|GetbIsAsyncrone)
    (AI|AIMoveTo OwnerController ControlledPawn (* (Class|BTFunctionLibrary|GetBlackboardValueasVector (Variables|Default|GetLocationKey)) 1.5) 0 (Variables|Default|GetStopDistance) false
      (:OnSuccess
        (AI|BehaviorTree|FinishExecute true))
      (:OnFail
        (AI|BehaviorTree|FinishExecute false)))
    (else
      (CallFunction|MovetoLocation OwnerController))))

(fn MovetoLocation
  (params (Controller :type AI%20Controller%20Object%20Reference))
  (bind _returnvalue (AI|Navigation|MovetoLocation Controller (Class|BTFunctionLibrary|GetBlackboardValueasVector (Variables|Default|GetLocationKey)) (Variables|Default|GetStopDistance) true true false true "/Script/AIModule.NavFilter_AIControllerDefault"))
  (switch Utilities|FlowControl|Switch|SwitchonEPathFollowingRequestResult _returnvalue
    (:Failed
      (AI|BehaviorTree|FinishExecute false :!label _label))
    (:AlreadyAtGoal
      (goto _label))
    (:RequestSuccessful
      (AI|BehaviorTree|FinishExecute true))))