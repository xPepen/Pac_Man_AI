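; Behavior tree task that moves the blue ghost's AI controller toward a target derived from the red ghost and the player, Pac-Man style.
; It takes a point slightly ahead of the player, then doubles the vector to it from the first BP_RedGhost found.
; It issues MoveToLocation and finishes successfully at once, without waiting for arrival or checking red ghost validity.
; An unused AIMoveTo node remains disconnected.
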(event EventReceiveExecuteAI
  (params (OwnerController :type AI%20Controller%20Object%20Reference) (ControlledPawn :type Pawn%20Object%20Reference))
  (bind _returnvalue (Game|GetPlayerController 0))
  (bind _redghost (CallFunction|GetRedGhostInfo))
  (bind _returnvalue_2 (Pawn|GetControlledPawn _returnvalue))
  (bind _returnvalue_3 (Transformation|GetActorLocation _redghost))
  ;[1 1 1] not sure for now need a map to test...
  (AI|Navigation|MovetoLocation OwnerController (+ _returnvalue_3 (* (- (+ (Transformation|GetActorLocation _returnvalue_2) (* (Transformation|GetActorForwardVector _returnvalue_2) (Math|Float|MakeLiteralFloat 1e+02))) _returnvalue_3) 2)) -1.0 true true false true 0)
  (AI|BehaviorTree|FinishExecute true))

(fn GetRedGhostInfo
  (bind _returnvalue (Actor|GetActorOfClass "/Game/Blueprint/Ghost/BP_RedGhost.BP_RedGhost_C"))
  (return (Utilities|IsValid _returnvalue) _returnvalue))