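; Behavior tree task that moves the yellow AI, apparently a ghost, either away on a wander or toward the player.
; After a short delay, it compares its distance to the player's pawn against a threshold.
; When close, it moves to a random navigable point around itself and finishes with the move's result; otherwise it starts a move to the player's location and finishes immediately.
; A red ghost lookup helper is defined but unused.
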(event EventReceiveExecuteAI
  (params (OwnerController :type AI%20Controller%20Object%20Reference) (ControlledPawn :type Pawn%20Object%20Reference))
  (bind _returnvalue (Transformation|GetActorLocation ControlledPawn))
  (bind _returnvalue_2 (Game|GetPlayerController 0))
  (bind _returnvalue_3 (Pawn|GetControlledPawn _returnvalue_2))
  (bind _returnvalue_4 (Transformation|GetActorLocation _returnvalue_3))
  (Utilities|FlowControl|Delay 0.5)
  (if (< (Math|Float|Absolute(Float) (Math|Vector|Distance(Vector) _returnvalue _returnvalue_4)) 8e+02)
    (bind _randomlocation (Class|NavigationSystemV1|GetRandomLocationinNavigableRadius _returnvalue 9e+02 0 0))
    (AI|AIMoveTo ControlledPawn _randomlocation 0 1e+02 false
      (:OnSuccess
        (AI|BehaviorTree|FinishExecute true))
      (:OnFail
        (AI|BehaviorTree|FinishExecute false)))
    (else
      (AI|Navigation|MovetoLocation OwnerController _returnvalue_4 -1.0 true true false true 0)
      (AI|BehaviorTree|FinishExecute true))))

(fn GetRedGhostInfo
  (bind _returnvalue (Actor|GetActorOfClass "/Game/Blueprint/Ghost/BP_RedGhost.BP_RedGhost_C"))
  (return (Utilities|IsValid _returnvalue) _returnvalue))